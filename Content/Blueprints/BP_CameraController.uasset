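; BP_CameraController drives a top-down camera with mouse drag panning and zooming.
; On BeginPlay it shows the cursor, enables click and hover events, and adds the Enhanced Input mapping context.
; Dragging offsets the actor by the mouse delta with screen axes swapped onto world X/Y, though CameraDragSpeed scales only Y.
; A separate input seeds the previous mouse position, and zoom inputs move the actor along world Z.
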(event Input|EnhancedActionEvents|EnhancedInputActionIA_OriginalLocation
  (params (ActionValue :type Boolean) (ElapsedSeconds :type Float%20%28double-precision%29) (TriggeredSeconds :type Float%20%28double-precision%29) (InputAction :type Input%20Action%20Object%20Reference :default "/Game/Blueprints/Input/IA_OriginalLocation.IA_OriginalLocation"))
  (bind _returnvalue (Class|WidgetLayoutLibrary|GetMousePositiononViewport))
  (Variables|Default|SetPreviousTouchLocation _returnvalue))

(event Input|EnhancedActionEvents|EnhancedInputActionIA_ZoomInCamera
  (params (ActionValue :type Boolean) (ElapsedSeconds :type Float%20%28double-precision%29) (TriggeredSeconds :type Float%20%28double-precision%29) (InputAction :type Input%20Action%20Object%20Reference :default "/Game/Blueprints/Input/IA_ZoomInCamera.IA_ZoomInCamera"))
  (Transformation|AddActorWorldOffset (Math|Vector|MakeVector 0.0 0.0 (Variables|Default|GetZoomInSpeed))))

(event Input|EnhancedActionEvents|EnhancedInputActionIA_DragCamera
  (params (ActionValue :type Boolean) (ElapsedSeconds :type Float%20%28double-precision%29) (TriggeredSeconds :type Float%20%28double-precision%29) (InputAction :type Input%20Action%20Object%20Reference :default "/Game/Blueprints/Input/IA_DragCamera.IA_DragCamera"))
  (bind _returnvalue (Class|WidgetLayoutLibrary|GetMousePositiononViewport))
  (Variables|Default|SetNewTouchLocation _returnvalue)
  (Transformation|AddActorWorldOffset (Math|Vector|MakeVector (.y (- (Variables|Default|GetNewTouchLocation) (Variables|Default|GetPreviousTouchLocation))) (* (.x (- (Variables|Default|GetNewTouchLocation) (Variables|Default|GetPreviousTouchLocation))) (Variables|Default|GetCameraDragSpeed)) 0.0))
  (Variables|Default|SetPreviousTouchLocation (Variables|Default|GetNewTouchLocation)))

(event Input|EnhancedActionEvents|EnhancedInputActionIA_ZoomOutCamera
  (params (ActionValue :type Boolean) (ElapsedSeconds :type Float%20%28double-precision%29) (TriggeredSeconds :type Float%20%28double-precision%29) (InputAction :type Input%20Action%20Object%20Reference :default "/Game/Blueprints/Input/IA_ZoomOutCamera.IA_ZoomOutCamera"))
  (Transformation|AddActorWorldOffset (Math|Vector|MakeVector 0.0 0.0 (Variables|Default|GetZoomOutSpeed))))

(event EventBeginPlay
  (CallFunction|CameraSetUp))

(event Collision|EventActorBeginOverlap
  (params (OtherActor :type Actor%20Object%20Reference)))

(event EventTick
  (params (DeltaSeconds :type Float%20%28single-precision%29)))

(fn ConstructionScript)

(fn CameraSetUp
  (bind _returnvalue (Game|GetPlayerController 0))
  (bind _returnvalue_2 (Game|GetPlayerController 0))
  (bind _returnvalue_3 (PlayerController|LocalPlayerSubsystems|GetEnhancedInputLocalPlayerSubsystem _returnvalue_2))
  (Variables|/Script/Engine.PlayerController|SetbShowMouseCursor _returnvalue true)
  (Variables|/Script/Engine.PlayerController|SetbEnableMouseOverEvents _returnvalue true)
  (Variables|/Script/Engine.PlayerController|SetbEnableClickEvents _returnvalue true)
  (Utilities|IsValid _returnvalue_3
    (:Is%20Valid
      (Input|AddMappingContext _returnvalue_3 "/Game/Blueprints/Input/IMC_TopDownCamera.IMC_TopDownCamera" 0 "(bIgnoreAllPressedKeysUntilRelease=True,bForceImmediately=False,bNotifyUserSettings=False)"))))