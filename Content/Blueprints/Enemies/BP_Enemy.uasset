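; Grid-based enemy actor that moves between tiles by picking at random from its possible actions.
; EnemyAction draws a tile from PossibleEnemyActions, then moves the actor there at unchanged height, updating its coordinates and both tiles' occupancy flags.
; Helpers look up tiles by coordinate in the tile manager and check occupancy.
; MakeEnemyActions only clears the action list; nothing here fills it.
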(event EventBeginPlay)

(event Collision|EventActorBeginOverlap
  (params (OtherActor :type Actor%20Object%20Reference)))

(event EventTick
  (params (DeltaSeconds :type Float%20%28single-precision%29)))

(fn ConstructionScript)

(fn EnemyAction
  (if (not (== (Utilities|Array|Length (Variables|Default|GetPossibleEnemyActions)) 0))
    (bind (_tilelocation _tileref) (CallFunction|DecideEnemyActions))
    (CallFunction|MoveEnemytoLocation _tilelocation _tileref)))

(fn CheckifTileExists
  (params (TileCoordinates :type Tile%20Location%20Structure%20Structure))
  (bind (_xcoordinate _ycoordinate) (Utilities|Struct|BreakTileLocationStructure TileCoordinates))
  (bind _array_element (Utilities|Array|ForEachLoopwithBreak (Variables|/Game/Blueprints/Tiles/BP_TileManager.BP_TileManager_C|GetTiles (Variables|Default|GetTileManagerRef)))
    (:LoopBody
      (if (== (and (== (.XCoordinate (Utilities|Struct|BreakTileLocationStructure (Variables|/Game/Blueprints/Tiles/BP_Tile.BP_Tile_C|GetTileCoordinates _array_element))) _xcoordinate) (== (.YCoordinate (Utilities|Struct|BreakTileLocationStructure (Variables|/Game/Blueprints/Tiles/BP_Tile.BP_Tile_C|GetTileCoordinates _array_element))) _ycoordinate)) true)
        (return true _array_element)))
    (:Completed
      (return false 0))))

(fn MoveEnemytoLocation
  (params (TileLocation :type Tile%20Location%20Structure%20Structure) (TileRef :type BP%20Tile%20Object%20Reference))
  (bind _returnvalue (Transformation|GetActorLocation TileRef))
  (Variables|/Game/Blueprints/Tiles/BP_Tile.BP_Tile_C|SetisOccupied (.TileRef (CallFunction|CheckifTileExists (Variables|Default|GetCurrentTileCoordinates))) false)
  (Transformation|SetActorLocation (Math|Vector|MakeVector (.x _returnvalue) (.y _returnvalue) (.z (Transformation|GetActorLocation))) false false)
  (Variables|Default|SetCurrentTileCoordinates TileLocation)
  (Variables|/Game/Blueprints/Tiles/BP_Tile.BP_Tile_C|SetisOccupied TileRef true))

(fn MakeEnemyActions
  (Utilities|Array|Clear (Variables|Default|GetPossibleEnemyActions)))

(fn DecideEnemyActions
  (bind _possibleenemyactions (Variables|Default|GetPossibleEnemyActions))
  (bind _possibleenemyactions_2 (Variables|Default|GetPossibleEnemyActions))
  (bind _returnvalue (Utilities|Array|Length _possibleenemyactions_2))
  (bind _returnvalue_2 (Math|Random|RandomInteger _returnvalue))
  (bind _output (Utilities|Array|Get(acopy) _possibleenemyactions _returnvalue_2))
  (bind (_tilecoordinates _tileref) (Utilities|Struct|BreakTileDataStructure _output))
  (return _tilecoordinates _tileref))

(fn CheckifTileOccupied
  (params (TileRef :type BP%20Tile%20Object%20Reference))
  (return (Variables|/Game/Blueprints/Tiles/BP_Tile.BP_Tile_C|GetisOccupied TileRef)))