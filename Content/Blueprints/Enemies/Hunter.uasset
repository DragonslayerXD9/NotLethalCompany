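; Hunter enemy for a tile-based game that roams the grid and lays traps on covered tiles.
; EnemyAction gathers existing, unoccupied orthogonal neighbours into PossibleEnemyActions, then defers to the parent implementation.
; Until TrapTriggered is set, it randomly tries to change the current tile's Event to a trap, pausing a turn after each success.
; RushTrap currently only skips trap-setting, with no movement bias toward the trap.
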(event EventBeginPlay
  (|CallParentFunction) ; This node is disabled and will not be called.\nDrag off pins to build functionality.
)

(event Collision|EventActorBeginOverlap
  (params (OtherActor :type Actor%20Object%20Reference))
  (|CallParentFunction OtherActor) ; This node is disabled and will not be called.\nDrag off pins to build functionality.
)

(event EventTick
  (params (DeltaSeconds :type Float%20%28single-precision%29))
  (|CallParentFunction DeltaSeconds) ; This node is disabled and will not be called.\nDrag off pins to build functionality.
)

(fn ConstructionScript
  (|CallParentFunction))

(fn EnemyAction
  (if (Variables|Default|GetTrapTriggered)
    (CallFunction|RushTrap)
    (else
      (CallFunction|StandardBehaviour)))
  (|CallParentFunction))

(fn RushTrap
  (CallFunction|MakeEnemyActions)
  (CallFunction|StandarMovement))

(fn StandardBehaviour
  (CallFunction|MakeEnemyActions)
  (if (Variables|Default|GetTrapJustSet)
    (Variables|Default|SetTrapJustSet false)
    (elif (== (Math|Random|RandomIntegerinRange 1 3) 3)
      (bind _wasplaced (CallFunction|SetTrap))
      (Variables|Default|SetTrapJustSet _wasplaced)))
  (CallFunction|StandarMovement))

(fn StandarMovement
  (bind _currenttilecoordinates (Variables|Default|GetCurrentTileCoordinates))
  (CallFunction|AddTiletoArray (Utilities|Struct|MakeTileLocationStructure (+ (.xcoordinate _currenttilecoordinates) 1) (.ycoordinate _currenttilecoordinates)))
  (CallFunction|AddTiletoArray (Utilities|Struct|MakeTileLocationStructure (- (.xcoordinate _currenttilecoordinates) 1) (.ycoordinate _currenttilecoordinates)))
  (CallFunction|AddTiletoArray (Utilities|Struct|MakeTileLocationStructure (.xcoordinate _currenttilecoordinates) (+ (.ycoordinate _currenttilecoordinates) 1)))
  (CallFunction|AddTiletoArray (Utilities|Struct|MakeTileLocationStructure (.xcoordinate _currenttilecoordinates) (- (.ycoordinate _currenttilecoordinates) 1))))

(fn SetTrap
  (bind _currenttilecoordinates (Variables|Default|GetCurrentTileCoordinates))
  (bind _tileref (CallFunction|CheckifTileExists _currenttilecoordinates))
  (if (Utilities|Enum|Equal(Enum) (Variables|/Game/Blueprints/Tiles/BP_Tile.BP_Tile_C|GetEvent _tileref) "NewEnumerator0")
    (if (Variables|/Game/Blueprints/Tiles/BP_Tile.BP_Tile_C|GetisUncovered _tileref)
      (return false)
      (else
        (Variables|/Game/Blueprints/Tiles/BP_Tile.BP_Tile_C|SetEvent _tileref "NewEnumerator3")
        (return true)))))

(fn AddTiletoArray
  (params (TileLocation :type Tile%20Location%20Structure%20Structure))
  (bind (_exists_ _tileref) (CallFunction|CheckifTileExists TileLocation))
  (if _exists_
    (bind _isoccupied (CallFunction|CheckifTileOccupied _tileref))
    (if (not _isoccupied)
      (Utilities|Array|Add (Variables|Default|GetPossibleEnemyActions) (Utilities|Struct|MakeTileDataStructure TileLocation _tileref)))))