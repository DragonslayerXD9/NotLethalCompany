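; KillerBugSpawn is a tile-grid enemy Blueprint that offers the four orthogonally adjacent tiles as its possible actions.
; Its EnemyAction override builds the options through MakeEnemyActions, then hands off to the parent implementation.
; MakeEnemyActions runs the parent version, then calls BadFunctionButWorks per direction, which adds each existing, unoccupied neighbour's coordinates and tile reference to PossibleEnemyActions.
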(event EventBeginPlay
  (|CallParentFunction) ; This node is disabled and will not be called.\nDrag off pins to build functionality.
)

(event Collision|EventActorBeginOverlap
  (params (OtherActor :type Actor%20Object%20Reference))
  (|CallParentFunction OtherActor) ; This node is disabled and will not be called.\nDrag off pins to build functionality.
)

(event EventTick
  (params (DeltaSeconds :type Float%20%28single-precision%29))
  (|CallParentFunction DeltaSeconds) ; This node is disabled and will not be called.\nDrag off pins to build functionality.
)

(fn ConstructionScript
  (|CallParentFunction))

(fn EnemyAction
  (CallFunction|MakeEnemyActions)
  (|CallParentFunction))

(fn MakeEnemyActions
  (|CallParentFunction)
  (CallFunction|BadFunctionButWorks 1)
  (CallFunction|BadFunctionButWorks 0 1)
  (CallFunction|BadFunctionButWorks -1)
  (CallFunction|BadFunctionButWorks 0 -1))

(fn BadFunctionButWorks
  (params (AddToX :type Integer) (AddToY :type Integer))
  (bind _currenttilecoordinates (Variables|Default|GetCurrentTileCoordinates))
  (bind _returnvalue (+ (.ycoordinate _currenttilecoordinates) AddToY))
  (bind _returnvalue_2 (+ (.xcoordinate _currenttilecoordinates) AddToX))
  (bind _tilelocationstructure (Utilities|Struct|MakeTileLocationStructure _returnvalue_2 _returnvalue))
  (bind (_exists_ _tileref) (CallFunction|CheckifTileExists _tilelocationstructure))
  (if _exists_
    (bind _isoccupied (CallFunction|CheckifTileOccupied _tileref))
    (if (not _isoccupied)
      (Utilities|Array|Add (Variables|Default|GetPossibleEnemyActions) (Utilities|Struct|MakeTileDataStructure _tilelocationstructure _tileref)))))