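; Berserker enemy for a tile-grid game that builds its candidate action tiles, switching to a longer-range berserk action every third turn.
; Standard turns collect the four orthogonal neighbours, then the parent EnemyAction runs.
; Berserk turns expand that set twice and trim the first two rings, leaving only tiles three steps away.
; AddTileToArray accepts only existing, unoccupied, unlisted tiles other than the current one.
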(event EventBeginPlay
  (|CallParentFunction)
  (Variables|Default|Settimer 0))

(event Collision|EventActorBeginOverlap
  (params (OtherActor :type Actor%20Object%20Reference))
  (|CallParentFunction OtherActor) ; This node is disabled and will not be called.\nDrag off pins to build functionality.
)

(event EventTick
  (params (DeltaSeconds :type Float%20%28single-precision%29))
  (|CallParentFunction DeltaSeconds) ; This node is disabled and will not be called.\nDrag off pins to build functionality.
)

(fn ConstructionScript
  (|CallParentFunction))

(fn EnemyAction
  (bind _output_get (Variables|Default|Settimer (+ (Variables|Default|Gettimer) 1)))
  (if (== _output_get 3)
    (Variables|Default|Settimer 0)
    (CallFunction|BerserkAction)
    (else
      (CallFunction|StandardAction)))
  (|CallParentFunction))

(fn AddSurroundingTiles
  (params (XAxis :type Integer) (YAxis :type Integer))
  (CallFunction|AddTiletoArray (Utilities|Struct|MakeTileLocationStructure (+ XAxis 1) YAxis))
  (CallFunction|AddTiletoArray (Utilities|Struct|MakeTileLocationStructure (- XAxis 1) YAxis))
  (CallFunction|AddTiletoArray (Utilities|Struct|MakeTileLocationStructure XAxis (+ YAxis 1)))
  (CallFunction|AddTiletoArray (Utilities|Struct|MakeTileLocationStructure XAxis (- YAxis 1))))

(fn StandardAction
  (bind _currenttilecoordinates (Variables|Default|GetCurrentTileCoordinates))
  (CallFunction|MakeEnemyActions)
  (CallFunction|AddSurroundingTiles (.xcoordinate _currenttilecoordinates) (.ycoordinate _currenttilecoordinates)))

(fn BerserkAction
  (bind _currenttilecoordinates (Variables|Default|GetCurrentTileCoordinates))
  (bind _possibleenemyactions (Variables|Default|GetPossibleEnemyActions))
  (bind _possibleenemyactions_2 (Variables|Default|GetPossibleEnemyActions))
  (bind _possibleenemyactions_3 (Variables|Default|GetPossibleEnemyActions))
  (CallFunction|MakeEnemyActions)
  (CallFunction|AddSurroundingTiles (.xcoordinate _currenttilecoordinates) (.ycoordinate _currenttilecoordinates))
  (bind _output_get (Variables|Default|SetarrayLength (- (Utilities|Array|Length _possibleenemyactions_2) 1)))
  (for _index (range 0 _output_get)
    (CallFunction|AddSurroundingTiles (.xcoordinate (.tilecoordinates (Utilities|Array|Get(acopy) _possibleenemyactions_2 _index))) (.ycoordinate (.tilecoordinates (Utilities|Array|Get(acopy) _possibleenemyactions_2 _index)))))
  (bind _output_get_2 (Variables|Default|SetarrayLength (- (Utilities|Array|Length _possibleenemyactions_3) 1)))
  (for _index_2 (range 0 _output_get_2)
    (CallFunction|AddSurroundingTiles (.xcoordinate (.tilecoordinates (Utilities|Array|Get(acopy) _possibleenemyactions_3 _index_2))) (.ycoordinate (.tilecoordinates (Utilities|Array|Get(acopy) _possibleenemyactions_3 _index_2)))))
  ;[1 1 1] Removing first few values ( of length 1 or 2) so berserk mode always travels 3
  (for _index_3 (range 0 (Variables|Default|GetarrayLength))
    (Utilities|Array|RemoveIndex _possibleenemyactions))
  (for _array_element _possibleenemyactions
    _))

(fn DoesntExistinList
  (params (TileSetIn :type Tile%20Location%20Structure%20Structure) (tile%20ref :type BP%20Tile%20Object%20Reference))
  (return (== (Utilities|Array|FindItem (Variables|Default|GetPossibleEnemyActions) (Utilities|Struct|MakeTileDataStructure TileSetIn tile%20ref)) -1) TileSetIn))

(fn IsOriginal
  (params (tileSetIn :type Tile%20Location%20Structure%20Structure))
  (bind (_xcoordinate _ycoordinate) (Utilities|Struct|BreakTileLocationStructure tileSetIn))
  (bind _currenttilecoordinates (Variables|Default|GetCurrentTileCoordinates))
  (return tileSetIn (== (and (== (.xcoordinate _currenttilecoordinates) _xcoordinate) (== (.ycoordinate _currenttilecoordinates) _ycoordinate)) true)))

(fn AddTiletoArray
  (params (TileLocation :type Tile%20Location%20Structure%20Structure))
  (bind (_exists_ _tileref) (CallFunction|CheckifTileExists TileLocation))
  (if _exists_
    (bind (_doesntexist _tilesetout) (CallFunction|DoesntExistinList TileLocation _tileref))
    (if _doesntexist
      (bind (_tilesetout_2 _original) (CallFunction|IsOriginal _tilesetout))
      (if (not _original)
        (bind _isoccupied (CallFunction|CheckifTileOccupied _tileref))
        (if (not _isoccupied)
          (Utilities|Array|Add (Variables|Default|GetPossibleEnemyActions) (Utilities|Struct|MakeTileDataStructure _tilesetout_2 _tileref)))))))