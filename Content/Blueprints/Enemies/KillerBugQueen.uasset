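; Killer bug queen enemy for a tile-grid game, which either lays an egg or gathers movement options on its turn.
; It has a one-in-three chance to lay, but never attempts it on the action right after a successful lay.
; An egg turns an event-free current tile into a delayed event, re-masking it if uncovered.
; Otherwise, it adds unoccupied orthogonal neighbors to PossibleEnemyActions before calling the parent EnemyAction.
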(event EventBeginPlay
  (Variables|Default|SetMonstertype "NewEnumerator3")
  (|CallParentFunction))

(event Collision|EventActorBeginOverlap
  (params (OtherActor :type Actor%20Object%20Reference))
  (|CallParentFunction OtherActor) ; This node is disabled and will not be called.\nDrag off pins to build functionality.
)

(event EventTick
  (params (DeltaSeconds :type Float%20%28single-precision%29))
  (|CallParentFunction DeltaSeconds) ; This node is disabled and will not be called.\nDrag off pins to build functionality.
)

(fn ConstructionScript
  (|CallParentFunction))

(fn EnemyAction
  (CallFunction|MakeEnemyActions)
  (if (Variables|Default|GetEggPlaced)
    (Variables|Default|SetEggPlaced false)
    (CallFunction|StadardMovement)
    (elif (== (Math|Random|RandomIntegerinRange 1 3) 3)
      (bind _wasplaced (CallFunction|PlaceEgg))
      (bind _output_get (Variables|Default|SetEggPlaced _wasplaced))
      (if _output_get
        _
        (else
          (CallFunction|StadardMovement :!label _label)))
      (else
        (goto _label))))
  (|CallParentFunction))

(fn PlaceEgg
  (bind _currenttilecoordinates (Variables|Default|GetCurrentTileCoordinates))
  (bind _tileref (CallFunction|CheckifTileExists _currenttilecoordinates))
  (if (Utilities|Enum|Equal(Enum) (Variables|/Game/Blueprints/Tiles/BP_Tile.BP_Tile_C|GetEvent _tileref) "NewEnumerator0")
    (if (Variables|/Game/Blueprints/Tiles/BP_Tile.BP_Tile_C|GetisUncovered _tileref)
      (Variables|/Game/Blueprints/Tiles/BP_Tile.BP_Tile_C|SetEvent _tileref "NewEnumerator6")
      (Variables|/Game/Blueprints/Tiles/BP_Tile.BP_Tile_C|SetRoundsTillEvent _tileref 4)
      (Rendering|Material|SetMaterial (Variables|/Game/Blueprints/Tiles/BP_Tile.BP_Tile_C|GetTile _tileref) 0 "/Game/Assets/Materials/Unknow.Unknow")
      (else
        (Variables|/Game/Blueprints/Tiles/BP_Tile.BP_Tile_C|SetEvent _tileref "NewEnumerator6")
        (Variables|/Game/Blueprints/Tiles/BP_Tile.BP_Tile_C|SetRoundsTillEvent _tileref 4)))
    (return true)))

(fn StadardMovement
  (bind _currenttilecoordinates (Variables|Default|GetCurrentTileCoordinates))
  (CallFunction|AddTiletoArray (Utilities|Struct|MakeTileLocationStructure (+ (.xcoordinate _currenttilecoordinates) 1) (.ycoordinate _currenttilecoordinates)))
  (CallFunction|AddTiletoArray (Utilities|Struct|MakeTileLocationStructure (- (.xcoordinate _currenttilecoordinates) 1) (.ycoordinate _currenttilecoordinates)))
  (CallFunction|AddTiletoArray (Utilities|Struct|MakeTileLocationStructure (.xcoordinate _currenttilecoordinates) (+ (.ycoordinate _currenttilecoordinates) 1)))
  (CallFunction|AddTiletoArray (Utilities|Struct|MakeTileLocationStructure (.xcoordinate _currenttilecoordinates) (- (.ycoordinate _currenttilecoordinates) 1))))

(fn AddTiletoArray
  (params (NewParam :type Tile%20Location%20Structure%20Structure))
  (bind (_exists_ _tileref) (CallFunction|CheckifTileExists NewParam))
  (if _exists_
    (bind _isoccupied (CallFunction|CheckifTileOccupied _tileref))
    (if (not _isoccupied)
      (Utilities|Array|Add (Variables|Default|GetPossibleEnemyActions) (Utilities|Struct|MakeTileDataStructure NewParam _tileref)))))