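; Swarm is a grid-based enemy that schedules a tile event, named as a spread, when it has room around it.
; On BeginPlay it sets its monster type; EnemyAction then gathers the existing, unoccupied orthogonal neighbor tiles into PossibleEnemyActions.
; If any exist, SpreadSwarm sets an event on the Swarm's current tile, not a neighbor, due in one round.
; The parent EnemyAction runs afterwards in either case.
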(event EventBeginPlay
  (Variables|Default|SetMonstertype "NewEnumerator6")
  (|CallParentFunction))

(event Collision|EventActorBeginOverlap
  (params (OtherActor :type Actor%20Object%20Reference))
  (|CallParentFunction OtherActor) ; This node is disabled and will not be called.\nDrag off pins to build functionality.
)

(event EventTick
  (params (DeltaSeconds :type Float%20%28single-precision%29))
  (|CallParentFunction DeltaSeconds) ; This node is disabled and will not be called.\nDrag off pins to build functionality.
)

(fn ConstructionScript
  (|CallParentFunction))

(fn EnemyAction
  (bind _currenttilecoordinates (Variables|Default|GetCurrentTileCoordinates))
  (CallFunction|MakeEnemyActions)
  (CallFunction|AddTiletoArray (Utilities|Struct|MakeTileLocationStructure (+ (.xcoordinate _currenttilecoordinates) 1) (.ycoordinate _currenttilecoordinates)))
  (CallFunction|AddTiletoArray (Utilities|Struct|MakeTileLocationStructure (- (.xcoordinate _currenttilecoordinates) 1) (.ycoordinate _currenttilecoordinates)))
  (CallFunction|AddTiletoArray (Utilities|Struct|MakeTileLocationStructure (.xcoordinate _currenttilecoordinates) (+ (.ycoordinate _currenttilecoordinates) 1)))
  (CallFunction|AddTiletoArray (Utilities|Struct|MakeTileLocationStructure (.xcoordinate _currenttilecoordinates) (- (.ycoordinate _currenttilecoordinates) 1)))
  (if (Utilities|Array|IsEmpty (Variables|Default|GetPossibleEnemyActions))
    _
    (else
      (CallFunction|SpreadSwarm)))
  (|CallParentFunction))

(fn AddTiletoArray
  (params (NewParam :type Tile%20Location%20Structure%20Structure))
  (bind (_exists_ _tileref) (CallFunction|CheckifTileExists NewParam))
  (if _exists_
    (bind _isoccupied (CallFunction|CheckifTileOccupied _tileref))
    (if (not _isoccupied)
      (Utilities|Array|Add (Variables|Default|GetPossibleEnemyActions) (Utilities|Struct|MakeTileDataStructure NewParam _tileref)))))

(fn SpreadSwarm
  (bind _currenttilecoordinates (Variables|Default|GetCurrentTileCoordinates))
  (bind _tileref (CallFunction|CheckifTileExists _currenttilecoordinates))
  (if true
    (Variables|/Game/Blueprints/Tiles/BP_Tile.BP_Tile_C|SetEvent _tileref "NewEnumerator10")
    (Variables|/Game/Blueprints/Tiles/BP_Tile.BP_Tile_C|SetRoundsTillEvent _tileref 1)))