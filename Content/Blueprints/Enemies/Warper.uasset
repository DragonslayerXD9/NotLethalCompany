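; Warper is a grid-based enemy that alternates standard steps with a periodic teleport on every third action.
; EnemyAction advances a counter, fills PossibleEnemyActions through StandardAction or TeleportAction, then calls the parent implementation.
; Standard actions offer existing, unoccupied orthogonal neighbour tiles.
; Teleport actions scan all TileManager tiles for unoccupied ones two to four steps away by Manhattan distance.
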(event EventBeginPlay
  (Variables|Default|SetMonstertype "NewEnumerator5")
  (|CallParentFunction)
  (Variables|Default|SetTimer 0))

(event Collision|EventActorBeginOverlap
  (params (OtherActor :type Actor%20Object%20Reference))
  (|CallParentFunction OtherActor) ; This node is disabled and will not be called.\nDrag off pins to build functionality.
)

(event EventTick
  (params (DeltaSeconds :type Float%20%28single-precision%29))
  (|CallParentFunction DeltaSeconds) ; This node is disabled and will not be called.\nDrag off pins to build functionality.
)

(fn ConstructionScript
  (|CallParentFunction))

(fn EnemyAction
  (bind _output_get (Variables|Default|Settimer (+ (Variables|Default|Gettimer) 1)))
  (if (== _output_get 3)
    (Variables|Default|Settimer 0)
    (CallFunction|TeleportAction)
    (else
      (CallFunction|StandardAction)))
  (|CallParentFunction))

(fn StandardAction
  (bind _currenttilecoordinates (Variables|Default|GetCurrentTileCoordinates))
  (CallFunction|MakeEnemyActions)
  (CallFunction|AddTiletoArray (Utilities|Struct|MakeTileLocationStructure (+ (.xcoordinate _currenttilecoordinates) 1) (.ycoordinate _currenttilecoordinates)))
  (CallFunction|AddTiletoArray (Utilities|Struct|MakeTileLocationStructure (- (.xcoordinate _currenttilecoordinates) 1) (.ycoordinate _currenttilecoordinates)))
  (CallFunction|AddTiletoArray (Utilities|Struct|MakeTileLocationStructure (.xcoordinate _currenttilecoordinates) (+ (.ycoordinate _currenttilecoordinates) 1)))
  (CallFunction|AddTiletoArray (Utilities|Struct|MakeTileLocationStructure (.xcoordinate _currenttilecoordinates) (- (.ycoordinate _currenttilecoordinates) 1))))

(fn TeleportAction
  (bind _tilemanagerref (Variables|Default|GetTileManagerRef))
  (bind _currenttilecoordinates (Variables|Default|GetCurrentTileCoordinates))
  (CallFunction|MakeEnemyActions)
  (for (_array_element _array_index) (Variables|/Game/Blueprints/Tiles/BP_TileManager.BP_TileManager_C|GetTiles _tilemanagerref)
    (if (not (Variables|/Game/Blueprints/Tiles/BP_Tile.BP_Tile_C|GetisOccupied _array_element))
      (if (and (> (+ (Math|Integer|Absolute(Integer) (- (.XCoordinate (Utilities|Struct|BreakTileLocationStructure (Utilities|Array|Get(acopy) (Variables|/Game/Blueprints/Tiles/BP_TileManager.BP_TileManager_C|GetSpawnedTileLocations _tilemanagerref) _array_index))) (.xcoordinate _currenttilecoordinates))) (Math|Integer|Absolute(Integer) (- (.YCoordinate (Utilities|Struct|BreakTileLocationStructure (Utilities|Array|Get(acopy) (Variables|/Game/Blueprints/Tiles/BP_TileManager.BP_TileManager_C|GetSpawnedTileLocations _tilemanagerref) _array_index))) (.ycoordinate _currenttilecoordinates)))) 1) (< (+ (Math|Integer|Absolute(Integer) (- (.XCoordinate (Utilities|Struct|BreakTileLocationStructure (Utilities|Array|Get(acopy) (Variables|/Game/Blueprints/Tiles/BP_TileManager.BP_TileManager_C|GetSpawnedTileLocations _tilemanagerref) _array_index))) (.xcoordinate _currenttilecoordinates))) (Math|Integer|Absolute(Integer) (- (.YCoordinate (Utilities|Struct|BreakTileLocationStructure (Utilities|Array|Get(acopy) (Variables|/Game/Blueprints/Tiles/BP_TileManager.BP_TileManager_C|GetSpawnedTileLocations _tilemanagerref) _array_index))) (.ycoordinate _currenttilecoordinates)))) 5))
        (Utilities|Array|Add (Variables|Default|GetPossibleEnemyActions) (Utilities|Struct|MakeTileDataStructure (Utilities|Array|Get(acopy) (Variables|/Game/Blueprints/Tiles/BP_TileManager.BP_TileManager_C|GetSpawnedTileLocations _tilemanagerref) _array_index) _array_element))))))

(fn AddTiletoArray
  (params (NewParam :type Tile%20Location%20Structure%20Structure))
  (bind (_exists_ _tileref) (CallFunction|CheckifTileExists NewParam))
  (if _exists_
    (bind _isoccupied (CallFunction|CheckifTileOccupied _tileref))
    (if (not _isoccupied)
      (Utilities|Array|Add (Variables|Default|GetPossibleEnemyActions) (Utilities|Struct|MakeTileDataStructure NewParam _tileref)))))