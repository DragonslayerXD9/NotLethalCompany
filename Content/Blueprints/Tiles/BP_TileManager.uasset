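; BP_TileManager builds the procedural tile map, places tile events and spawns enemies.
; GenerateMap clears old tiles, then grows a random walk from a random starter tile over part of a grid, backtracking at dead ends.
; Distance from the starter sets each tile's zone level and material.
; Events and random enemies pick zones by weighted roll favoring outer zones; events fall back to other zones, enemies seek unoccupied tiles.
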(event EventBeginPlay)

(event Collision|EventActorBeginOverlap
  (params (OtherActor :type Actor%20Object%20Reference)))

(event EventTick
  (params (DeltaSeconds :type Float%20%28single-precision%29)))

(fn ConstructionScript)

(fn SpawnEnemy
  (bind (_sumofrates1 _tileswithrates) (CallFunction|SetTileRatesforZones 2.0 5.0 1e+01))
  (bind _keys (Utilities|Map|Keys _tileswithrates))
  (LocalVariables|SetTileRarity (Math|Random|RandomFloatinRange 0.0 _sumofrates1))
  (bind _array_element (Utilities|Array|ForEachLoopwithBreak _keys :!label _label)
    (:LoopBody
      (if (< (LocalVariables|GetTileRarity) (.Value (Utilities|Map|Find _tileswithrates _array_element)))
        (bind _output (CallFunction|GetRandomTilebyZoneLevelwithNoMonsters _array_element))
        (goto _label Break)
        (else
          (LocalVariables|SetTileRarity (- (LocalVariables|GetTileRarity) (.Value (Utilities|Map|Find _tileswithrates _array_element)))))))
    (:Completed
      (bind _returnvalue (Game|SpawnActorfromClass (CallFunction|SelectRandomEnemy) (Math|Transform|MakeTransform (Transformation|GetActorLocation _output)) "Undefined" "MultiplyWithRoot" 0 0))
      (Variables|/Game/Blueprints/Enemies/BP_Enemy.BP_Enemy_C|SetTileManagerRef _returnvalue self)
      (Variables|/Game/Blueprints/Enemies/BP_Enemy.BP_Enemy_C|SetCurrentTileCoordinates _returnvalue (Variables|/Game/Blueprints/Tiles/BP_Tile.BP_Tile_C|GetTileCoordinates _output))
      (return _returnvalue))))

(fn SelectRandomEnemy
  (bind _spawnableenemies (Variables|Default|GetSpawnableEnemies))
  (return (Utilities|Array|Get(acopy) _spawnableenemies (Math|Random|RandomInteger (Utilities|Array|Length _spawnableenemies)))))

(fn GenerateGrid
  (params (Width :type Integer) (Height :type Integer))
  (for _index (range 0 (- Height 1))
    (for _index_2 (range 0 (- Width 1))
      (Utilities|Array|Add (Variables|Default|GetGridLocations) (Utilities|Struct|MakeTileLocationStructure _index_2 _index)))))

(fn SpawnTile
  (params (TileCoordinates :type Tile%20Location%20Structure%20Structure))
  (bind (_xcoordinate _ycoordinate) (Utilities|Struct|BreakTileLocationStructure TileCoordinates))
  (Variables|Default|SetTilesToSpawn (- (Variables|Default|GetTilesToSpawn) 1))
  (bind _returnvalue (Game|SpawnActorfromClass "/Game/Blueprints/Tiles/BP_Tile.BP_Tile_C" (Math|Transform|MakeTransform (Math|Vector|MakeVector (Math|Conversions|ToFloat(Integer) (* _ycoordinate (Variables|Default|GetDistanceBetweenTiles))) (Math|Conversions|ToFloat(Integer) (* _xcoordinate (Variables|Default|GetDistanceBetweenTiles))) 0.0)) "Undefined" "MultiplyWithRoot" 0 0))
  (Variables|/Game/Blueprints/Tiles/BP_Tile.BP_Tile_C|SetTileManagerRef _returnvalue self)
  (bind _output_get (Variables|/Game/Blueprints/Tiles/BP_Tile.BP_Tile_C|SetTileCoordinates _returnvalue TileCoordinates))
  (Utilities|Array|Add (Variables|Default|GetTiles) _returnvalue)
  (CallFunction|EstablishTileZoneLevel _returnvalue)
  (Utilities|Array|Add (Variables|Default|GetSpawnedTileLocations) _output_get)
  (return _output_get _returnvalue))

(fn GenerateMap
  (CallFunction|ResetMap)
  (CallFunction|GenerateGrid (Variables|Default|GetWidth) (Variables|Default|GetHeight))
  (CallFunction|CalculateAmountOfTiles 0.7 0.8)
  (CallFunction|SpawnStarterTile)
  (CallFunction|GeneratetheRestOftheMap)
  (CallFunction|AddEventstoTiles))

(fn SpawnStarterTile
  (bind _gridlocations (Variables|Default|GetGridLocations))
  (bind _output_get (LocalVariables|SetTmpTileCoordinates (Utilities|Array|Get(acopy) _gridlocations (Math|Random|RandomInteger (Utilities|Array|Length _gridlocations)))))
  (bind (_tilespawnlocation _returnvalue) (CallFunction|SpawnTile _output_get))
  (bind _output_get_2 (Variables|Default|SetStarterTile _returnvalue))
  (Rendering|Material|SetMaterial (Variables|/Game/Blueprints/Tiles/BP_Tile.BP_Tile_C|GetTile _output_get_2) 0 "/Game/Assets/Materials/StartZone.StartZone")
  (return _tilespawnlocation))

(fn IsLocationinGrid
  (params (TileCoordinates :type Tile%20Location%20Structure%20Structure))
  (return (Utilities|Array|ContainsItem (Variables|Default|GetGridLocations) TileCoordinates)))

(fn IsLocationonExistingTile
  (params (TileCoordinates :type Tile%20Location%20Structure%20Structure))
  (for _array_element (Variables|Default|GetTiles)
    (if (CallFunction|CompareTileCoordinates (Variables|/Game/Blueprints/Tiles/BP_Tile.BP_Tile_C|GetTileCoordinates _array_element) TileCoordinates)
      (return true)))
  (return false))

(fn EstablishTileZoneLevel
  (params (Tile :type BP%20Tile%20Object%20Reference))
  (bind _startertile (Variables|Default|GetStarterTile))
  (bind _tilecoordinates (Variables|/Game/Blueprints/Tiles/BP_Tile.BP_Tile_C|GetTileCoordinates _startertile))
  (LocalVariables|SetTileRef Tile)
  (Utilities|IsValid (Variables|Default|GetStarterTile)
    (:Is%20Valid
      (if (<= (CallFunction|CalculateVectorLength (.xcoordinate (Variables|/Game/Blueprints/Tiles/BP_Tile.BP_Tile_C|GetTileCoordinates (LocalVariables|GetTileRef))) (.ycoordinate (Variables|/Game/Blueprints/Tiles/BP_Tile.BP_Tile_C|GetTileCoordinates (LocalVariables|GetTileRef))) (.xcoordinate _tilecoordinates) (.ycoordinate _tilecoordinates)) (Math|Float|Sqrt 8.0))
        (Variables|/Game/Blueprints/Tiles/BP_Tile.BP_Tile_C|SetZoneLevel (LocalVariables|GetTileRef) "NewEnumerator0")
        (Rendering|Material|SetMaterial (Variables|/Game/Blueprints/Tiles/BP_Tile.BP_Tile_C|GetTile (LocalVariables|GetTileRef)) 0 "/Game/Assets/Materials/Zone1.Zone1")
        (elif (<= (CallFunction|CalculateVectorLength (.xcoordinate (Variables|/Game/Blueprints/Tiles/BP_Tile.BP_Tile_C|GetTileCoordinates (LocalVariables|GetTileRef))) (.ycoordinate (Variables|/Game/Blueprints/Tiles/BP_Tile.BP_Tile_C|GetTileCoordinates (LocalVariables|GetTileRef))) (.xcoordinate _tilecoordinates) (.ycoordinate _tilecoordinates)) (Math|Float|Sqrt 24.0))
          (Variables|/Game/Blueprints/Tiles/BP_Tile.BP_Tile_C|SetZoneLevel (LocalVariables|GetTileRef) "NewEnumerator1")
          (Rendering|Material|SetMaterial (Variables|/Game/Blueprints/Tiles/BP_Tile.BP_Tile_C|GetTile (LocalVariables|GetTileRef)) 0 "/Game/Assets/Materials/Zone2.Zone2")
          (else
            (Variables|/Game/Blueprints/Tiles/BP_Tile.BP_Tile_C|SetZoneLevel (LocalVariables|GetTileRef) "NewEnumerator2")
            (Rendering|Material|SetMaterial (Variables|/Game/Blueprints/Tiles/BP_Tile.BP_Tile_C|GetTile (LocalVariables|GetTileRef)) 0 "/Game/Assets/Materials/Zone3.Zone3")))))))

(fn GeneratetheRestOftheMap
  (if (> (Variables|Default|GetTilesToSpawn) 0) :!label _label
    (bind _possibletileplacementcoordinates1 (CallFunction|GetPossibleDirections (Utilities|Array|Get(acopy) (Variables|Default|GetSpawnedTileLocations) (LocalVariables|GetCurrentTileIdx)) :!label _label_2))
    (if (> (Utilities|Array|Length _possibletileplacementcoordinates1) 0)
      (CallFunction|SpawnTile (Utilities|Array|Get(acopy) _possibletileplacementcoordinates1 (Math|Random|RandomInteger (Utilities|Array|Length _possibletileplacementcoordinates1))))
      (LocalVariables|SetCurrentTileIdx (- (Utilities|Array|Length (Variables|Default|GetSpawnedTileLocations)) 1))
      (goto _label)
      (else
        (LocalVariables|SetCurrentTileIdx (- (LocalVariables|GetCurrentTileIdx) 1))
        (if (> (LocalVariables|GetCurrentTileIdx) 0)
          (goto _label_2)
          (else
            (return)))))))

(fn GetPossibleDirections
  (params (CurrentTileCoordinates :type Tile%20Location%20Structure%20Structure))
  (bind (_xcoordinate _ycoordinate) (Utilities|Struct|BreakTileLocationStructure CurrentTileCoordinates))
  (for _array_element (LocalVariables|GetStandardTileGenerationDirections)
    (bind _locationingrid_ (CallFunction|IsLocationinGrid (Utilities|Struct|MakeTileLocationStructure (+ _xcoordinate (.xcoordinate (.ToMoveCoordinates (Utilities|Struct|BreakTileMovementGenerationStructure _array_element)))) (+ (.ycoordinate (.ToMoveCoordinates (Utilities|Struct|BreakTileMovementGenerationStructure _array_element))) _ycoordinate))))
    (if (== _locationingrid_ true)
      (bind _tilealreadyexists_ (CallFunction|IsLocationonExistingTile (Utilities|Struct|MakeTileLocationStructure (+ _xcoordinate (.xcoordinate (.ToMoveCoordinates (Utilities|Struct|BreakTileMovementGenerationStructure _array_element)))) (+ (.ycoordinate (.ToMoveCoordinates (Utilities|Struct|BreakTileMovementGenerationStructure _array_element))) _ycoordinate))))
      (if (not (== _tilealreadyexists_ true))
        (Utilities|Array|Add (LocalVariables|GetPossibleDirections) (.GenerationDirection (Utilities|Struct|BreakTileMovementGenerationStructure _array_element)))
        (Utilities|Array|Add (LocalVariables|GetPossibleTilePlacementCoordinates) (Utilities|Struct|MakeTileLocationStructure (+ _xcoordinate (.xcoordinate (.ToMoveCoordinates (Utilities|Struct|BreakTileMovementGenerationStructure _array_element)))) (+ (.ycoordinate (.ToMoveCoordinates (Utilities|Struct|BreakTileMovementGenerationStructure _array_element))) _ycoordinate))))))
  (return (LocalVariables|GetPossibleDirections) (LocalVariables|GetPossibleTilePlacementCoordinates)))

(fn SetTileRatesforZones
  (params (ZoneOneRate :type Float%20%28double-precision%29) (ZoneTwoRate :type Float%20%28double-precision%29) (ZoneThreeRate :type Float%20%28double-precision%29))
  (bind _output_get (LocalVariables|SetTileZonesWithRates (Utilities|Map|MakeMap "NewEnumerator0" ZoneOneRate "NewEnumerator1" ZoneTwoRate "NewEnumerator2" ZoneThreeRate)))
  (bind _values (Utilities|Map|Values _output_get))
  (for _array_element _values
    (bind _output_get_2 (LocalVariables|SetSumOfRates (+ _array_element (LocalVariables|GetSumOfRates)))))
  (return _output_get_2 _output_get))

(fn AddEventstoTiles
  (bind _possibletileevents1 (CallFunction|GetPossibleEvents))
  (LocalVariables|SetEventsToAdd _possibletileevents1)
  (bind (_sumofrates1 _tileswithrates) (CallFunction|SetTileRatesforZones 2.0 5.0 1e+01))
  (bind _keys (Utilities|Map|Keys _tileswithrates))
  (for _index (range 0 (- (Utilities|Array|Length (LocalVariables|GetEventsToAdd)) 1))
    (LocalVariables|SetTileRarity (Math|Random|RandomFloatinRange 0.0 _sumofrates1))
    (bind _array_element (Utilities|Array|ForEachLoopwithBreak _keys :!label _label)
      (:LoopBody
        (if (< (LocalVariables|GetTileRarity) (.Value (Utilities|Map|Find _tileswithrates _array_element)))
          (bind _tileforevents (CallFunction|GetRandomTilebyZoneLevelwithNoEvent _array_element))
          (Variables|/Game/Blueprints/Tiles/BP_Tile.BP_Tile_C|SetEvent _tileforevents (Utilities|Array|Get(acopy) (LocalVariables|GetEventsToAdd) _index))
          (goto _label Break)
          (else
            (LocalVariables|SetTileRarity (- (LocalVariables|GetTileRarity) (.Value (Utilities|Map|Find _tileswithrates _array_element))))))))))

(fn CalculateAmountOfTiles
  (params (Min :type Float%20%28double-precision%29) (Max :type Float%20%28double-precision%29))
  (Variables|Default|SetTilesToSpawn (Math|Float|Round (* (* (Variables|Default|GetWidth) (Variables|Default|GetHeight)) (Math|Random|RandomFloatinRange Min Max))))
  (return))

(fn GetRandomTilebyZoneLevelwithNoEvent
  (params (ZoneLevel :type TileZoneLevels%20Enum :default "NewEnumerator3"))
  (bind _tmpzonelevels (LocalVariables|GetTmpZoneLevels))
  (bind _returnvalue (Utilities|Array|Length _tmpzonelevels))
  (LocalVariables|SetTmpZoneLevel ZoneLevel)
  (bind _output_get (LocalVariables|SetTempTiles (Variables|Default|GetTiles)))
  (Utilities|Array|Shuffle _output_get)
  (for _array_element (LocalVariables|GetTempTiles) :!label _label
    (if (Utilities|Enum|Equal(Enum) (LocalVariables|GetTmpZoneLevel) (Variables|/Game/Blueprints/Tiles/BP_Tile.BP_Tile_C|GetZoneLevel _array_element))
      (if (Utilities|Enum|Equal(Enum) (Variables|/Game/Blueprints/Tiles/BP_Tile.BP_Tile_C|GetEvent _array_element) "NewEnumerator0")
        (return _array_element))))
  ;[1 1 1] Security Mechanism
  (Utilities|Array|RemoveItem _tmpzonelevels (LocalVariables|GetTmpZoneLevel))
  (if (> _returnvalue 0)
    (Development|PrintString "You're not running away from me boy!!!")
    (LocalVariables|SetTmpZoneLevel (Utilities|Array|Get(acopy) _tmpzonelevels (Math|Random|RandomInteger _returnvalue)))
    (goto _label)))

(fn GetRandomTilebyZoneLevel
  (params (ZoneLevel :type TileZoneLevels%20Enum :default "NewEnumerator3"))
  (LocalVariables|SetTmpZoneLevel ZoneLevel)
  (bind _output_get (LocalVariables|SetTmpTiles (Variables|Default|GetTiles)))
  (Utilities|Array|Shuffle _output_get)
  (for _array_element (LocalVariables|GetTmpTiles)
    (if (Utilities|Enum|Equal(Enum) (LocalVariables|GetTmpZoneLevel) (Variables|/Game/Blueprints/Tiles/BP_Tile.BP_Tile_C|GetZoneLevel _array_element))
      (return _array_element))))

(fn GetRandomTilewithNoEvent
  (params (Tiles :type Array%20of%20BP%20Tile%20Object%20References))
  (bind _returnvalue (Utilities|Array|Length Tiles))
  (bind _returnvalue_2 (Math|Random|RandomInteger _returnvalue))
  (bind _output (Utilities|Array|Get(acopy) Tiles _returnvalue_2))
  (return _output (Utilities|Enum|Equal(Enum) (Variables|/Game/Blueprints/Tiles/BP_Tile.BP_Tile_C|GetEvent _output) "NewEnumerator0")))

(fn GetPossibleEvents
  (bind _possibletileevents (LocalVariables|GetPossibleTileEvents))
  (bind _possibletileevents_2 (LocalVariables|GetPossibleTileEvents))
  (bind _events (LocalVariables|GetEvents))
  (for _index (range 1 (Variables|Default|GetAmountOfTreasure))
    (Utilities|Array|Add _possibletileevents_2 "NewEnumerator1"))
  (for _index_2 (range 0 6)
    (bind _output_get (LocalVariables|SetTmpEvent (Utilities|Array|Get(acopy) _events (Math|Random|RandomInteger (Utilities|Array|Length _events)))))
    (Utilities|Array|Add _possibletileevents_2 _output_get)
    (if (Utilities|Enum|Equal(Enum) (LocalVariables|GetTmpEvent) "NewEnumerator5")
      (Utilities|Array|Add (LocalVariables|GetPossibleTileEvents) "NewEnumerator5")))
  (Utilities|Array|Shuffle _possibletileevents)
  (return _possibletileevents))

(fn ResetMap
  (bind _startertile (Variables|Default|GetStarterTile))
  (Utilities|Array|Clear (Variables|Default|GetTiles))
  (Utilities|Array|Clear (Variables|Default|GetSpawnedTileLocations))
  (Utilities|Array|Clear (Variables|Default|GetGridLocations))
  (bind _outactors (Actor|GetAllActorsOfClass "/Game/Blueprints/Tiles/BP_Tile.BP_Tile_C"))
  (for _array_element _outactors
    (Utilities|IsValid _array_element
      (:Is%20Valid
        (Default|DestroySelf _array_element))))
  (Utilities|IsValid _startertile
    (:Is%20Valid
      (Actor|DestroyActor _startertile))))

(fn GetRandomTilebyZoneLevelwithNoMonsters
  (params (ZoneLevel :type TileZoneLevels%20Enum :default "NewEnumerator3"))
  (LocalVariables|SetTmpZoneLevel ZoneLevel)
  (bind _output_get (LocalVariables|SetTmpTiles (Variables|Default|GetTiles)))
  (Utilities|Array|Shuffle _output_get)
  (for _array_element (LocalVariables|GetTmpTiles)
    (if (and (Utilities|Enum|Equal(Enum) (LocalVariables|GetTmpZoneLevel) (Variables|/Game/Blueprints/Tiles/BP_Tile.BP_Tile_C|GetZoneLevel _array_element)) (== (Variables|/Game/Blueprints/Tiles/BP_Tile.BP_Tile_C|GetisOccupied _array_element) false))
      (return _array_element))))

(fn CalculateVectorLength
  (params (X1 :type Integer) (Y1 :type Integer) (X2 :type Integer) (Y2 :type Integer))
  (return (Math|Float|Sqrt (Math|Conversions|ToFloat(Integer) (+ (Math|Float|Square (Math|Conversions|ToFloat(Integer) (- X1 X2))) (Math|Float|Square (Math|Conversions|ToFloat(Integer) (- Y1 Y2))))))))