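; Clickable grid tile that hides an event (treasure, bear, mud or warp trap, egg), revealed by material swap on click.
; Hovering toggles a highlight overlay, clicking an occupied tile prints its monster, and clicking bear traps or eggs sets RoundsTillEvent to one.
; TileEvent clears bear traps and eggs showing their material; other eggs spawn a KillerBugSpawn with tile manager and coordinates, or wait while occupied.
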(event OnBeginCursorOver(Tile)
  (params (TouchedComponent :type Primitive%20Component%20Object%20Reference))
  (Rendering|Material|SetOverlayMaterial (Variables|Default|GetTile) "/Game/Assets/Materials/M_HighlightMaterial.M_HighlightMaterial" :!class /Script/Engine.MeshComponent))

(event OnEndCursorOver(Tile)
  (params (TouchedComponent :type Primitive%20Component%20Object%20Reference))
  (Rendering|Material|SetOverlayMaterial (Variables|Default|GetTile) 0 :!class /Script/Engine.MeshComponent))

(event EventBeginPlay)

(event Collision|EventActorBeginOverlap
  (params (OtherActor :type Actor%20Object%20Reference)))

(event EventTick
  (params (DeltaSeconds :type Float%20%28single-precision%29)))

(event MouseInput|EventActorOnClicked
  (params (ButtonPressed :type Key%20Structure))
  (bind _tile (Variables|Default|GetTile))
  (if (Variables|Default|GetisOccupied)
    (Development|PrintString (Utilities|String|EnumtoString (Variables|Default|GetMonster)))
    (elif (Variables|Default|GetisUncovered)
      (switch Utilities|FlowControl|Switch|SwitchonTileEvents (Variables|Default|GetEvent)
        (:NewEnumerator3
          (Rendering|Material|SetMaterial (Variables|Default|GetTile) 0 "/Game/Assets/Materials/BearTrap.BearTrap"))
        (:NewEnumerator6
          (Rendering|Material|SetMaterial (Variables|Default|GetTile) 0 "/Game/StarterContent/Materials/M_Brick_Clay_Beveled.M_Brick_Clay_Beveled")))
      (Variables|Default|SetRoundsTillEvent 1)
      (else
        (Variables|Default|SetisUncovered true)
        (switch Utilities|FlowControl|Switch|SwitchonTileEvents (Variables|Default|GetEvent)
          (:NewEnumerator0
            (if (Utilities|Enum|NotEqual(Enum) (Variables|Default|GetZoneLevel) "NewEnumerator3")
              (Rendering|Material|SetMaterial _tile 0 "/Game/Assets/Materials/Empty.Empty")))
          (:NewEnumerator1
            (Rendering|Material|SetMaterial _tile 0 "/Game/Assets/Materials/Tresure.Tresure"))
          (:NewEnumerator3
            (Rendering|Material|SetMaterial _tile 0 "/Game/Assets/Materials/BearTrap.BearTrap")
            (Variables|Default|SetRoundsTillEvent 1))
          (:NewEnumerator4
            (Rendering|Material|SetMaterial _tile 0 "/Game/Assets/Materials/Mud.Mud"))
          (:NewEnumerator5
            (Rendering|Material|SetMaterial _tile 0 "/Game/Assets/Materials/Warp.Warp"))
          (:NewEnumerator6
            (Rendering|Material|SetMaterial _tile 0 "/Game/StarterContent/Materials/M_Brick_Clay_Beveled.M_Brick_Clay_Beveled")
            (Variables|Default|SetRoundsTillEvent 1)))))))

(fn ConstructionScript)

(fn DestroySelf
  (Actor|DestroyActor))

(fn TileEvent
  (params (NewParam :type BP%20Tile%20Manager%20Object%20Reference))
  (switch Utilities|FlowControl|Switch|SwitchonTileEvents (Variables|Default|GetEvent)
    (:NewEnumerator3
      (Rendering|Material|SetMaterial (Variables|Default|GetTile) 0 "/Game/Assets/Materials/Empty.Empty" :!label _label)
      (Variables|Default|SetEvent "NewEnumerator0" :!label _label_2)
      (return (stale _newparam1)))
    (:NewEnumerator6
      (if (== (Rendering|Material|GetMaterial (Variables|Default|GetTile) 0) "/Game/StarterContent/Materials/M_Brick_Clay_Beveled.M_Brick_Clay_Beveled")
        (goto _label)
        (elif (Variables|Default|GetisOccupied)
          (Variables|Default|SetRoundsTillEvent 1)
          (else
            (bind _newparam1 (CallFunction|SpawnBug NewParam))
            (if (Variables|Default|GetisUncovered)
              (goto _label)
              (else
                (goto _label_2)))))))))

(fn SpawnBug
  (params (NewParam :type BP%20Tile%20Manager%20Object%20Reference))
  (bind _returnvalue (Game|SpawnActorfromClass "/Game/Blueprints/Enemies/KillerBugSpawn.KillerBugSpawn_C" (Math|Transform|MakeTransform (Transformation|GetActorLocation)) "Undefined" "MultiplyWithRoot" 0 0))
  (Variables|/Game/Blueprints/Enemies/BP_Enemy.BP_Enemy_C|SetTileManagerRef _returnvalue NewParam)
  (Variables|/Game/Blueprints/Enemies/BP_Enemy.BP_Enemy_C|SetCurrentTileCoordinates _returnvalue (Variables|Default|GetTileCoordinates))
  (Variables|Default|SetisOccupied true)
  (return _returnvalue))